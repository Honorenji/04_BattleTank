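; Player-controlled tank pawn that hands its barrel, turret and tracks to aiming and movement logic on BeginPlay.
; Aim axes rotate an azimuth gimbal and spring arm to orbit the view.
; Driving supports direct per-track throttles or forward and turn intents routed through the TankMovement component, and the Fire action calls Fire.
; Left Bracket rights the tank by zeroing pitch and roll while keeping yaw.
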(event `self.ReceiveBeginPlay`
  (`self.SetBarrelReference` (`self.Barrel`))
  (`self.SetTurretReference` (`self.Turret`))
  (`TankMovementComponent.Initialise` (`self.TankMovement`) (`self.Track_l`) (`self.Track_r`)))

(event `InputAxis|AimAzimuth`
  (params (AxisValue :type "Float (single-precision)"))
  ;[1 0.2 0 0] Aim Input Binding
  (`SceneComponent.K2_AddLocalRotation` (`self.Azimuth Gimbal`) (`KismetMathLibrary.MakeRotator` 0.0 0.0 AxisValue) false false))

(event `InputAxis|Left Track Throttle`
  (params (AxisValue :type "Float (single-precision)"))
  ;[1 0.2 0 0] Movement Input Binding
  (`TankTrack.SetThrottle` (`self.Track_l`) AxisValue))

(event `InputAxis|AimElevation`
  (params (AxisValue :type "Float (single-precision)"))
  ;[1 0.2 0 0] Aim Input Binding
  (`SceneComponent.K2_AddLocalRotation` (`self.SpringArm`) (`KismetMathLibrary.MakeRotator` 0.0 AxisValue) false false))

(event `InputAxis|Right Track Throttle`
  (params (AxisValue :type "Float (single-precision)"))
  ;[1 0.2 0 0] Movement Input Binding
  (`TankTrack.SetThrottle` (`self.Track_r`) AxisValue))

(event `InputAxis|MoveForward`
  (params (AxisValue :type "Float (single-precision)"))
  ;[1 0.2 0 0] Movement Input Binding
  (`TankMovementComponent.IntendMoveForward` (`self.TankMovement`) AxisValue))

(event `InputAction|Fire`
  (params (Key :type "Key Structure" :default "AnyKey"))
  ;[1 0.2 0 0] Aim Input Binding
  (:`Pressed`
    (`self.Fire`)))

(event `InputAxis|TurnRight`
  (params (AxisValue :type "Float (single-precision)"))
  ;[1 0.2 0 0] Movement Input Binding
  (`TankMovementComponent.IntendTurnRight` (`self.TankMovement`) AxisValue))

(event `Key|LeftBracket`
  (params (Key :type "Key Structure" :default "AnyKey"))
  (bind (_returnvalue_roll _returnvalue_pitch _returnvalue_yaw) (`KismetMathLibrary.BreakRotator` (`self.K2_GetActorRotation`)))
  (:`Pressed`
    (`self.K2_SetActorRotation` (`KismetMathLibrary.MakeRotator` 0.0 0.0 _returnvalue_yaw))))

(fn `UserConstructionScript`)
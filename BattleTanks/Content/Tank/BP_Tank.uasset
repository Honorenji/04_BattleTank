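; Player-controllable tank pawn that wires its barrel, turret and tracks into TankAiming and TankMovement components at BeginPlay.
; Input forwards driving intent to TankMovement and firing to TankAiming, while aim axes rotate an azimuth gimbal and spring arm separately.
; A camera action toggles third- and first-person views, and a hard-bound Left Bracket key rights the tank by keeping only its yaw.
; The health bar widget receives a reference to the tank.
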(event `self.ReceiveBeginPlay`
  (`TankAimingComponent.Initialise` (`self.TankAiming`) (`self.Barrel`) (`self.Turret`))
  (`TankMovementComponent.Initialise` (`self.TankMovement`) (`self.Track_l`) (`self.Track_r`))
  (`self.InitialiseHealthBarWidget`))

(event `InputAxis|AimAzimuth`
  (params (AxisValue :type "Float (single-precision)"))
  ;[1 0.2 0 0] Aim Input Binding
  (`SceneComponent.K2_AddLocalRotation` (`self.Azimuth Gimbal`) (`KismetMathLibrary.MakeRotator` 0.0 0.0 AxisValue) false false))

(event `InputAxis|MoveForward`
  (params (AxisValue :type "Float (single-precision)"))
  ;[1 0.2 0 0] Movement Input Binding
  (`TankMovementComponent.IntendMoveForward` (`self.TankMovement`) AxisValue))

(event `InputAxis|AimElevation`
  (params (AxisValue :type "Float (single-precision)"))
  ;[1 0.2 0 0] Aim Input Binding
  (`SceneComponent.K2_AddLocalRotation` (`self.SpringArm`) (`KismetMathLibrary.MakeRotator` 0.0 AxisValue) false false))

(event `InputAxis|TurnRight`
  (params (AxisValue :type "Float (single-precision)"))
  ;[1 0.2 0 0] Movement Input Binding
  (`TankMovementComponent.IntendTurnRight` (`self.TankMovement`) AxisValue))

(event `InputAction|Fire`
  (params (Key :type "Key Structure" :default "AnyKey"))
  ;[1 0.2 0 0] Aim Input Binding
  (:`Pressed`
    (`TankAimingComponent.Fire` (`self.TankAiming`))))

(event `Key|LeftBracket`
  (params (Key :type "Key Structure" :default "AnyKey"))
  (bind (_returnvalue_roll _returnvalue_pitch _returnvalue_yaw) (`KismetMathLibrary.BreakRotator` (`self.K2_GetActorRotation`)))
  (:`Pressed`
    (`self.K2_SetActorRotation` (`KismetMathLibrary.MakeRotator` 0.0 0.0 _returnvalue_yaw))))

(event `InputAction|SwapCamera`
  (params (Key :type "Key Structure" :default "AnyKey"))
  (:`Pressed`
    (`ActorComponent.ToggleActive` (`self.3rd Person`))
    (`ActorComponent.ToggleActive` (`self.1st Person`))))

(fn `InitialiseHealthBarWidget`
  (bind _aswbp_health_bar (cast `/Game/Widgets/WBP_HealthBar` (`WidgetComponent.GetUserWidgetObject` (`self.Widget`))))
  (set `/Game/Widgets/WBP_HealthBar.TankRef` self _aswbp_health_bar))

(fn `UserConstructionScript`)